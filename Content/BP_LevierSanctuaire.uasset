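; BP_LevierSanctuaire is a sanctuary lever that opens the referenced SanctuaryDoor when the player interacts with it.
; Entering its Box trigger clears the player controller's OnInteraction bindings and binds a new event, while leaving restores the character's default interaction.
; The Interact event opens the door and calls DisableBox on its Text reference.
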(event `Interact`
  (`/Game/FirstPersonBP/Blueprints/SomeBlueprints/BP_LeftDoor.OpenDoor` (`self.SanctuaryDoor`))
  (`/Game/FirstPersonBP/Blueprints/Widget/BP_Text.DisableBox` (`self.Text`)))

(event `self.Box.OnComponentBeginOverlap`
  (params (OverlappedComponent :type "PrimitiveComponent Object Reference") (OtherActor :type "Actor Object Reference") (OtherComp :type "PrimitiveComponent Object Reference") (OtherBodyIndex :type Integer) (bFromSweep :type Boolean) (SweepResult :type "HitResult Structure (by ref)"))
  (bind _mainplayercontroller (`/Game/FirstPersonBP/Blueprints/Manager/BPFL_CallPlayerController.CallMainPlayerController`))
  (clear `/Game/FirstPersonBP/Blueprints/Manager/BP_PC_MainPlayerController.OnInteraction` _mainplayercontroller)
  (add `/Game/FirstPersonBP/Blueprints/Manager/BP_PC_MainPlayerController.OnInteraction` _mainplayercontroller (`|CreateDelegate` :!event `Interact`)))

(event `self.Box.OnComponentEndOverlap`
  (params (OverlappedComponent :type "PrimitiveComponent Object Reference") (OtherActor :type "Actor Object Reference") (OtherComp :type "PrimitiveComponent Object Reference") (OtherBodyIndex :type Integer))
  (`/Game/FirstPersonBP/Blueprints/Character/BP_PersoPrincipal.DefautInteraction` (`/Game/FirstPersonBP/Blueprints/Manager/BPFL_CallPlayerController.CallMainPlayerCharacter`)))

(fn `UserConstructionScript`)